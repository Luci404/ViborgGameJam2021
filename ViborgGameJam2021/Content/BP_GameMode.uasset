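; Game mode for a local multiplayer game with a shared BP_Camera view, per-character lives and a UI.
; On BeginPlay it creates a player for each PlayerStart, matching numeric tags to indices, then possesses a spawned character and removes CameraActors.
; ResetGame resets the UI and restores each character's lives, alive state and ragdoll strength.
; Reset teleports characters to starts by array order, whereas spawning matches by tag.
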(event `self.ReceiveBeginPlay`
  (bind _outactors (`GameplayStatics.GetAllActorsOfClass` "/Game/BP_Camera.BP_Camera_C"))
  (set `self.CameraRef` (`|GetArrayItem` _outactors))
  (bind _outactors_2 (`GameplayStatics.GetAllActorsOfClass` "/Script/Engine.PlayerStart"))
  (set `self.PlayerStartArray` _outactors_2)
  (`self.SpawnInputReceivers`)
  (bind _returnvalue (`|CreateWidget` "/Game/BP_UI.BP_UI_C"))
  (bind _output_get (set `self.UI` _returnvalue))
  (`UserWidget.AddToViewport` _output_get 0))

(fn `RemoveUnusedCameras`
  (bind _outactors (`GameplayStatics.GetAllActorsOfClass` "/Script/Engine.CameraActor"))
  (for _array_element _outactors
    (`self.K2_DestroyActor` _array_element)))

(fn `ResetGame`
  (`/Game/BP_UI.ResetUI` (`self.UI`))
  (bind _outactors (`GameplayStatics.GetAllActorsOfClass` "/Game/BP_Character.BP_Character_C"))
  (for _array_element _outactors
    (set `/Game/BP_Character.PlayerLives` 3 _array_element)
    (set `/Game/BP_Character.bIsAlive` true _array_element)
    (bind _outactors_2 (`GameplayStatics.GetAllActorsOfClass` "/Script/Engine.PlayerStart"))
    (`self.K2_SetActorTransform` _array_element (`self.GetTransform` (`|GetArrayItem` _outactors_2 (`/Game/BP_Character.Index` _array_element))) false true)
    (`/Game/BP_Ragdoll_Actor.Set_Strength` (`/Game/BP_Ragdoll_Component.BP_Ragdoll` (`/Game/BP_Character.Ragdoll_Component` _array_element)) 1.5)
    (set `/Game/BP_Character.bIsAlive` true _array_element)))

(fn `SpawnInputReceivers`
  (locals (Index :type Integer))
  (bind _returnvalue (`GameplayStatics.GetPlayerController` (`local.Index`)))
  (for (_ _array_index) (`self.PlayerStartArray`)
    (set `local.Index` _array_index)
    (for _array_element (`self.PlayerStartArray`)
      (if (== (`KismetStringLibrary.Conv_StringToInt` (`KismetStringLibrary.Conv_NameToString` (`PlayerStart.PlayerStartTag` _array_element))) (`local.Index`))
        (`GameplayStatics.CreatePlayer` -1)
        (bind _returnvalue_2 (`|SpawnActorFromClass` "/Game/BP_Character.BP_Character_C" (`self.GetTransform` (`|GetArrayItem` (`self.PlayerStartArray`) (`local.Index`))) "Undefined" "OverrideRootScale" null (`local.Index`) null))
        (`KismetArrayLibrary.Array_AddUnique` (`self.PlayerInputReceiverArray`) _returnvalue_2)
        (`Controller.Possess` _returnvalue _returnvalue_2)
        (`KismetArrayLibrary.Array_AddUnique` (`self.PlayerControllerArray`) _returnvalue)
        (`PlayerController.SetViewTargetWithBlend` (`GameplayStatics.GetPlayerController` (`local.Index`)) (`self.CameraRef`) 0.0 "VTBlend_Linear" 0.0 false)))
    (`self.RemoveUnusedCameras`)))

(fn `UserConstructionScript`)