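; BP_InputReceiver lets a player join the game by pressing Start, spawning and possessing a character for that player.
; It reads BP_GameMode's start, controller and camera references, spawning at the start matching its PlayerIndex, possessing it with that controller and setting the view to the shared camera.
; A disconnected earlier version spawning at the receiver's own transform remains unused.
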(event `InputAction|Start`
  (params (Key :type "Key Structure"))
  (bind _playerindex (`self.PlayerIndex`))
  (:`Pressed`
    (bind _asbp_game_mode (cast `/Game/BP_GameMode` (`GameplayStatics.GetGameMode`)))
    (bind _returnvalue (`|SpawnActorFromClass` "/Game/BP_Character.BP_Character_C" (`self.GetTransform` (`|GetArrayItem` (`/Game/BP_GameMode.PlayerStartArray` _asbp_game_mode) _playerindex)) "Undefined" "OverrideRootScale" null _playerindex null))
    (bind _output (`|GetArrayItem` (`/Game/BP_GameMode.PlayerControllerArray` _asbp_game_mode) _playerindex))
    (`Controller.Possess` _output _returnvalue)
    (`PlayerController.SetViewTargetWithBlend` _output (`/Game/BP_GameMode.CameraRef` _asbp_game_mode) 0.0 "VTBlend_Linear" 0.0 false)))

(fn `UserConstructionScript`)