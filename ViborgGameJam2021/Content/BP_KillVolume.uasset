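; Kill volume that respawns a BP_Character that enters its box and costs it lives.
; On overlap it prints the touching component's name and acts only when that component is the character's capsule, ignoring its other components.
; It then teleports the character above a randomly picked PlayerStart, calls RemoveLives and applies a timed Knockout.
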(event `self.Box.OnComponentBeginOverlap`
  (params (OverlappedComponent :type "PrimitiveComponent Object Reference") (OtherActor :type "Actor Object Reference") (OtherComp :type "PrimitiveComponent Object Reference") (OtherBodyIndex :type Integer) (bFromSweep :type Boolean) (SweepResult :type "HitResult Structure (by ref)"))
  (bind _asbp_character (cast `/Game/BP_Character` OtherActor))
  (`KismetSystemLibrary.PrintString` (`KismetSystemLibrary.GetDisplayName` OtherComp))
  (if (== (`Character.CapsuleComponent` _asbp_character) OtherComp)
    (bind _outactors (`GameplayStatics.GetAllActorsOfClass` "/Script/Engine.PlayerStart"))
    (bind _returnvalue (`self.GetTransform` (`|GetArrayItem` _outactors (`KismetMathLibrary.RandomIntegerInRange` 0 (- (`KismetArrayLibrary.Array_Length` _outactors) 1)))))
    (`self.K2_SetActorTransform` OtherActor (`KismetMathLibrary.MakeTransform` (`KismetMathLibrary.MakeVector` (.x (.location _returnvalue)) (.y (.location _returnvalue)) (+ (.z (.location _returnvalue)) 500.0)) (.rotation _returnvalue) (.scale _returnvalue)) false true)
    (`/Game/BP_Character.Remove Lives` _asbp_character)
    (`/Game/BP_Character.Knockout` _asbp_character 3.0)))

(fn `UserConstructionScript`)