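; BP_Lift is a lift actor that moves vertically when something overlaps its trigger sphere.
; The overlap plays a timeline from the start, with a Moving flag ignoring new overlaps until it finishes.
; Each update resets the root to the position cached at BeginPlay, then adds the track value as a Z offset, teleporting without sweep so the curve defines absolute height.
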(event `self.ReceiveBeginPlay`
  (bind _output_get (set `self.StartPosition` (`SceneComponent.K2_GetComponentLocation` (`self.DefaultSceneRoot`)))))

(event `self.Sphere.OnComponentBeginOverlap`
  (params (OverlappedComponent :type "PrimitiveComponent Object Reference") (OtherActor :type "Actor Object Reference") (OtherComp :type "PrimitiveComponent Object Reference") (OtherBodyIndex :type Integer) (bFromSweep :type Boolean) (SweepResult :type "HitResult Structure (by ref)"))
  (bind _defaultsceneroot (`self.DefaultSceneRoot`))
  (if (not (`self.Moving`))
    (set `self.Moving` true)
    (bind (_direction _newtrack_0) (`Timeline|Timeline_0` :!via `PlayFromStart`)
      (:`Update`
        (`SceneComponent.K2_SetWorldLocation` _defaultsceneroot (stale `self.ReceiveBeginPlay` _output_get) false true)
        (`SceneComponent.K2_AddWorldOffset` _defaultsceneroot (`KismetMathLibrary.MakeVector` 0.0 0.0 _newtrack_0) false true))
      (:`Finished`
        (set `self.Moving` false)))))

(fn `UserConstructionScript`)