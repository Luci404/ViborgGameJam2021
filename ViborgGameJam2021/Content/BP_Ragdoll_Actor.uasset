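; Actor that turns a player pawn into an active ragdoll that moves with character movement and grabs with both hands.
; Boot events add a PhysicalAnimationComponent and simulate the mesh, with adjustable strength.
; Each tick, hand sphere traces drive physics handles that hold movable static or skeletal meshes, or pin the hand to non-movable ones.
; Tick also feeds movement velocity to the pelvis, blending Z, while the capsule follows the pelvis.
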(event `Boot_Events`
  (params (player_pawn :type "Pawn Object Reference"))
  ;[1 1 1] boot actor reference, and also set simulate his dynamic physics
  (bind _output_get (set `self.player_pawn` player_pawn))
  (bind _returnvalue (`self.GetComponentByClass` _output_get "/Script/Engine.SkeletalMeshComponent"))
  (`/Engine/EditorBlueprintResources/StandardMacros.IsValid` _returnvalue
    (:`Is Valid`
      (set `self.mesh` _returnvalue))
    (:`Is Not Valid`
      _))
  (bind _returnvalue_2 (`self.GetComponentByClass` _output_get "/Script/Engine.CharacterMovementComponent"))
  (`/Engine/EditorBlueprintResources/StandardMacros.IsValid` _returnvalue_2
    (:`Is Valid`
      (set `self.char_movement` _returnvalue_2))
    (:`Is Not Valid`
      _))
  (bind _returnvalue_3 (`AddComponent|NODE_AddPhysicalAnimationComponent-0` :`self` (`self.player_pawn`)))
  (bind _output_get_2 (set `self.physical_animation` _returnvalue_3))
  (`PhysicalAnimationComponent.SetSkeletalMeshComponent` _output_get_2 (`self.Mesh`))
  (if (== (`self.physics_profile`) "None")
    (`PhysicalAnimationComponent.ApplyPhysicalAnimationSettingsBelow` (`self.physical_animation`) "root" (make `PhysicalAnimationData` true (`self.Orientation_Strength`) (`self.Angular_Velocity_Strength`) 0.0 0.0 (`self.Max_Linear_Force`) (`self.Max_Angular_Force`)) false)
    (else
      (`PhysicalAnimationComponent.ApplyPhysicalAnimationProfileBelow` (`self.physical_animation`) "root" (`self.physics_profile`) false false)))
  (`SkeletalMeshComponent.SetConstraintProfile` (`self.Mesh`) "pelvis" (`self.constraint_profile`) true)
  (`PrimitiveComponent.SetSimulatePhysics` (`self.Mesh`) true))

(event `self.ReceiveTick`
  (params (DeltaSeconds :type "Float (single-precision)"))
  ;[1 1 1] on tick trace both hands, and set velocity of character
  (`self.trace_hold` "hand_l")
  (`self.trace_hold` "hand_r" "NewEnumerator1")
  (`self.set_velocity`))

(event `Boot_Values`
  (params (Orientation_Strength :type "Float (double-precision)") (Angular_Velocity_Strength :type "Float (double-precision)") (Max_Linear_Force :type "Float (double-precision)") (Max_Angular_Force :type "Float (double-precision)") (Ragdoll_Strength :type "Float (double-precision)") (physics_profile :type Name) (constraint_profile :type Name))
  ;[1 1 1] boot physical values
  (set `self.Orientation_Strength` Orientation_Strength)
  (set `self.Angular_Velocity_Strength` Angular_Velocity_Strength)
  (set `self.Max_Linear_Force` Max_Linear_Force)
  (set `self.Max_Angular_Force` Max_Angular_Force)
  (set `self.Ragdoll_Strength` Ragdoll_Strength)
  (set `self.physics_profile` physics_profile)
  (set `self.constraint_profile` constraint_profile))

(event `Grab`
  (params (Enum :type "/Game/Enum_Ragdoll_Hands Enum" :default "NewEnumerator0"))
  ;[1 1 1] grab and release events
  (switch `/Game/Enum_Ragdoll_Hands` Enum
    (:`NewEnumerator0`
      (set `self.hold_l` true)
      (bind _returnvalue (`AddComponent|NODE_AddPhysicsHandleComponent-0`))
      (set `self.handle_l` _returnvalue))
    (:`NewEnumerator1`
      (set `self.hold_r` true)
      (bind _returnvalue_2 (`AddComponent|NODE_AddPhysicsHandleComponent-1`))
      (set `self.handle_r` _returnvalue_2))))

(event `Set_Strength`
  (params (Ragdoll_Strength :type "Float (double-precision)"))
  ;[1 1 1] update ragdoll strength, clamped by 0 to 100
  (bind _output_get (set `self.Ragdoll_Strength` Ragdoll_Strength))
  (`PhysicalAnimationComponent.SetStrengthMultiplyer` (`self.physical_animation`) (`KismetMathLibrary.FClamp` _output_get 0.0 100.0)))

(event `Release`
  (params (Enum :type "/Game/Enum_Ragdoll_Hands Enum" :default "NewEnumerator0"))
  ;[1 1 1] grab and release events
  (switch `/Game/Enum_Ragdoll_Hands` Enum
    (:`NewEnumerator0`
      (set `self.hold_l` false)
      (`ActorComponent.K2_DestroyComponent` (`self.handle_l`))
      (set `self.handle_l` null)
      (set `self.grabbed_l` false)
      (set `self.static_l` false))
    (:`NewEnumerator1`
      (set `self.hold_r` false)
      (`ActorComponent.K2_DestroyComponent` (`self.handle_r`))
      (set `self.handle_r` null)
      (set `self.grabbed_r` false)
      (set `self.static_r` false))))

(fn `set_velocity`
  (bind _z (.z (`SceneComponent.GetSocketLocation` (`self.Mesh`) "pelvis")))
  (bind _z_2 (.z (`MovementComponent.Velocity` (`self.char_movement`))))
  ;[1 1 1] gets char movement velocity and sets it as pelvis velocity, also clamps the Z velocity by pelvis + - 100 and sets as capsule location
  ; so it mixed character movement with physical pelvis, and nevers lets it go far away from it
  (`SceneComponent.K2_SetWorldLocation` (`self.K2_GetRootComponent` (`self.player_pawn`)) (`KismetMathLibrary.MakeVector` (.x (`SceneComponent.GetSocketLocation` (`self.Mesh`) "pelvis")) (.y (`SceneComponent.GetSocketLocation` (`self.Mesh`) "pelvis")) (`KismetMathLibrary.FClamp` (.z (`SceneComponent.K2_GetComponentLocation` (`self.K2_GetRootComponent` (`self.player_pawn`)))) (- _z 100.0) (+ _z 100.0))) false false) ; set world location of capsule\nto update it by pelvis location\nso if we push any physical actor\nhis capsule will be moved also
  (bind _returnvalue (`PrimitiveComponent.GetPhysicsLinearVelocity` (`self.Mesh`) "pelvis"))
  (bind _z_3 (.z _returnvalue))
  (`PrimitiveComponent.SetPhysicsLinearVelocity` (`self.Mesh`) (`KismetMathLibrary.MakeVector` (.x (`MovementComponent.Velocity` (`self.char_movement`))) (.y (`MovementComponent.Velocity` (`self.char_movement`))) (`KismetMathLibrary.Lerp` _z_3 _z_2 (`KismetMathLibrary.SelectFloat` 0.0 0.5 (< _z_2 _z_3)))) false "pelvis"))

(fn `trace_hold`
  (params (hand :type Name) (Enum :type "/Game/Enum_Ragdoll_Hands Enum" :default "NewEnumerator0"))
  (locals (hand_location :type "Vector Structure") (hand_name :type Name) (static_location :type "Vector Structure") (local_enum :type "/Game/Enum_Ragdoll_Hands Enum"))
  (bind _local_enum (`local.local_enum`))
  (bind _returnvalue (select `/Game/Enum_Ragdoll_Hands` (`local.local_enum`) :`NewEnumerator0` (`self.handle_l`) :`NewEnumerator1` (`self.handle_r`)))
  (bind _returnvalue_2 (select `/Game/Enum_Ragdoll_Hands` (`local.local_enum`) :`NewEnumerator0` (`self.handle_l`) :`NewEnumerator1` (`self.handle_r`)))
  ;[1 1 1] trace check for each hand, while holding grab, to grab different logic with different components, like skeletals, static with physics, or just static meshes
  ; shortly a grabbing logic
  (set `local.local_enum` Enum)
  (if (select `/Game/Enum_Ragdoll_Hands` (`local.local_enum`) :`NewEnumerator0` (`self.hold_l`) :`NewEnumerator1` (`self.hold_r`))
    (bind _output_get (set `local.hand_name` hand))
    (bind _returnvalue_3 (`SceneComponent.GetSocketLocation` (`self.mesh`) _output_get))
    (bind _output_get_2 (set `local.hand_location` _returnvalue_3))
    (bind _outhit (`KismetSystemLibrary.SphereTraceSingle` _output_get_2 (- _returnvalue_3 (0.0 0.0 40.0)) 25.0 "TraceTypeQuery1" false (`|MakeArray` (`self.player_pawn`) :!type "Actor Object Reference") (`self.Draw_Debug`))) ; spheric trace from hands, by radius 25
    (if (select `/Game/Enum_Ragdoll_Hands` (`local.local_enum`) :`NewEnumerator0` (`self.grabbed_l`) :`NewEnumerator1` (`self.grabbed_r`))
      (`PhysicsHandleComponent.SetTargetLocation` _returnvalue_2 (`local.hand_location`))
      (elif (select `/Game/Enum_Ragdoll_Hands` (`local.local_enum`) :`NewEnumerator0` (`self.static_l`) :`NewEnumerator1` (`self.static_r`))
        (`PhysicsHandleComponent.SetTargetLocation` _returnvalue_2 (select `/Game/Enum_Ragdoll_Hands` (`local.local_enum`) :`NewEnumerator0` (`self.static_left`) :`NewEnumerator1` (`self.static_right`)))
        (else
          (bind (_bblockinghit _binitialoverlap _time _distance _location _impactpoint _normal _impactnormal _physmat _hitactor _hitcomponent _hitbonename) (`GameplayStatics.BreakHitResult` _outhit))
          (bind _asstatic_mesh_component (cast `StaticMeshComponent` _hitcomponent)
            (:`then`
              (if (`|EnumEquality` (`SceneComponent.Mobility` _asstatic_mesh_component) "Movable")
                (`PhysicsHandleComponent.GrabComponentAtLocation` _returnvalue _asstatic_mesh_component _hitbonename _impactpoint)
                (switch `/Game/Enum_Ragdoll_Hands` _local_enum :!label _label ; set booleans for static and grabbed
                  (:`NewEnumerator0`
                    (set `self.grabbed_l` true))
                  (:`NewEnumerator1`
                    (set `self.grabbed_r` true)))
                (else
                  (`PhysicsHandleComponent.GrabComponentAtLocation` _returnvalue (`self.mesh`) (`local.hand_name`) _impactpoint)
                  (switch `/Game/Enum_Ragdoll_Hands` _local_enum
                    (:`NewEnumerator0`
                      (set `self.static_l` true)
                      (set `self.static_left` _impactpoint) ; save static locations, as grapple points
                    )
                    (:`NewEnumerator1`
                      (set `self.static_r` true)
                      (set `self.static_right` _impactpoint))))))
            (:`CastFailed`
              (bind _asskeletal_mesh_component (cast `SkeletalMeshComponent` _hitcomponent)) ; if not static check if it is skeletal meshe, if so then grab it by hit bone
              (`PhysicsHandleComponent.GrabComponentAtLocation` _returnvalue _asskeletal_mesh_component _hitbonename _impactpoint)
              (goto _label))))))))

(fn `UserConstructionScript`)