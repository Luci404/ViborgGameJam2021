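; Actor component that gives its owning Pawn ragdoll behavior by delegating to a separate BP_Ragdoll_Actor.
; On BeginPlay it always spawns that actor at the world origin and stores a reference to it.
; It passes its physical-animation style settings (strengths, force limits, physics and constraint profiles) through BootValues, then hands the owner to BootEvents if it is a Pawn.
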(event `self.ReceiveBeginPlay`
  ;[1 1 1] boot ragdoll actor
  (bind _returnvalue (`|SpawnActorFromClass` "/Game/BP_Ragdoll_Actor.BP_Ragdoll_Actor_C" (`KismetMathLibrary.MakeTransform` (0.0 0.0 0.0)) "AlwaysSpawn" "OverrideRootScale" null null))
  (bind _output_get (set `self.BP_Ragdoll` _returnvalue))
  (`/Game/BP_Ragdoll_Actor.Boot_Values` _output_get (`self.Orientation_Strength`) (`self.Angular_Velocity_Strength`) (`self.Max_Linear_Force`) (`self.Max_Angular_Force`) (`self.Ragdoll_Strength`) (`self.Physics_Profile`) (`self.Constraint_Profile`))
  (bind _aspawn (cast `Pawn` (`self.GetOwner`)))
  (`/Game/BP_Ragdoll_Actor.Boot_Events` (`self.BP_Ragdoll`) _aspawn))